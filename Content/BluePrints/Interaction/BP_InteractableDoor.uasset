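; Interactable hinged door that players toggle, and that enemies can open when allowed, swinging away or toward based on the opener's local X position.
; A looping timer, rather than Tick, lerps DoorPivot yaw over OpenDuration, blocking interaction while moving.
; Motion end updates the prompt and arms an optional auto-close timer, which manual interaction cancels.
; TryOpenForEnemy reuses OnInteract, then overrides swing direction from the enemy's side.
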(event Custom|AutoCloseDoor
  ;[0.15 0.15 0.15 0.5] One auto-close timer per door. Arm after fully open; cancel on manual interaction. Callback rechecks state and starts the shared motion timer.
  (Utilities|Time|ClearTimerbyFunctionName 0 "AutoCloseDoor")
  (if (and (and (Variables|Default|GetIsOpen) (not (Variables|Default|GetIsMoving))) (Variables|Door|AutoClose|GetisAutoClose))
    (Variables|Default|SetStartYaw (Variables|Default|GetTargetYaw))
    (Variables|Default|SetIsOpen false)
    (Variables|Default|SetTargetYaw 0.0)
    (Variables|Default|SetMotionStartTime (Utilities|Time|GetTimeSeconds))
    (Variables|Default|SetIsMoving true)
    (Utilities|Time|SetTimerbyFunctionName 0 "UpdateDoorMotion" 0.016 true)))

(event Custom|StartAutoCloseTimer
  ;[0.15 0.15 0.15 0.5] One auto-close timer per door. Arm after fully open; cancel on manual interaction. Callback rechecks state and starts the shared motion timer.
  (Utilities|Time|ClearTimerbyFunctionName 0 "AutoCloseDoor")
  (if (and (and (Variables|Default|GetIsOpen) (Variables|Door|AutoClose|GetisAutoClose)) (not (Variables|Default|GetIsMoving)))
    (Utilities|Time|SetTimerbyFunctionName 0 "AutoCloseDoor" (Math|Float|Max(Float) (Variables|Door|AutoClose|GetAutoCloseDelay) 0.05))))

(event EventBeginPlay
  (|CallParentFunction) ; This node is disabled and will not be called.\nDrag off pins to build functionality.
)

(event Collision|EventActorBeginOverlap
  (params (OtherActor :type Actor%20Object%20Reference))
  (|CallParentFunction OtherActor) ; This node is disabled and will not be called.\nDrag off pins to build functionality.
)

(event EventTick
  (params (DeltaSeconds :type Float%20%28single-precision%29))
  (|CallParentFunction DeltaSeconds) ; This node is disabled and will not be called.\nDrag off pins to build functionality.
)

(fn ConstructionScript
  (|CallParentFunction))

(fn OnInteract
  (params (InteractingPlayer :type BP%20Player%20Character%20Object%20Reference))
  (|CallParentFunction InteractingPlayer)
  (Utilities|IsValid InteractingPlayer
    (:Is%20Valid
      ;[0.15 0.15 0.15 0.5] Cancel the old auto-close countdown before every accepted manual transition.
      (Utilities|Time|ClearTimerbyFunctionName 0 "AutoCloseDoor")
      (Variables|Default|SetStartYaw (Variables|Default|GetTargetYaw))
      (Variables|Default|SetIsOpen (not (Variables|Default|GetIsOpen)))
      (bind _directionsign (CallFunction|CalculateOpenDirection InteractingPlayer))
      (bind _output_get (Variables|Default|SetOpenDirectionSign _directionsign))
      (Variables|Default|SetTargetYaw (* (Math|Float|SelectFloat (Variables|Door|GetOpenAngle) 0.0 (Variables|Default|GetIsOpen)) _output_get))
      (Variables|Default|SetMotionStartTime (Utilities|Time|GetTimeSeconds))
      (Variables|Default|SetIsMoving true)
      (Utilities|Time|SetTimerbyFunctionName 0 "UpdateDoorMotion" 0.016 true))
    (:Is%20Not%20Valid
      (Development|PrintString "Player is None"))))

(fn CanInteractwith
  (params (InteractingPlayer :type BP%20Player%20Character%20Object%20Reference))
  ;[0.15 0.15 0.15 0.5] Keep parent requirements and ignore repeated interaction while the door is moving.
  (return (and (|CallParentFunction InteractingPlayer) (not (Variables|Default|GetIsMoving)))))

(fn UpdateDoorMotion
  (bind _returnvalue (Utilities|Time|GetTimeSeconds))
  (bind _motionstarttime (Variables|Default|GetMotionStartTime))
  (bind _openduration (Variables|Door|GetOpenDuration))
  (bind _returnvalue_2 (Math|Float|Max(Float) _openduration 0.05))
  (bind _returnvalue_3 (- _returnvalue _motionstarttime))
  (bind _returnvalue_4 (/ _returnvalue_3 _returnvalue_2))
  (bind _returnvalue_5 (Math|Float|Clamp(Float) _returnvalue_4))
  ;[0.15 0.15 0.15 0.5] Interpolate hinge yaw over OpenDuration. Stop the timer at the exact target and update the next action prompt.
  (CallFunction|ApplyDoorRotation (Math|Float|Lerp (Variables|Default|GetStartYaw) (Variables|Default|GetTargetYaw) _returnvalue_5))
  (if (>= _returnvalue_5 1.0)
    (Utilities|Time|ClearTimerbyFunctionName 0 "UpdateDoorMotion")
    (Variables|Default|SetIsMoving false)
    (CallFunction|StartAutoCloseTimer)
    (Variables|Default|SetInteractionName (Utilities|Text|ToText(String) (Utilities|String|SelectString "Close door" "Open door" (Variables|Default|GetIsOpen)))))
  (return))

(fn ApplyDoorRotation
  (params (currentYaw :type Float%20%28double-precision%29))
  (Transformation|SetRelativeRotation (Variables|Default|GetDoorPivot) (Math|Rotator|MakeRotator 0.0 0.0 currentYaw) false false)
  (return true))

(fn CalculateOpenDirection
  (params (InteractingPlayer :type BP%20Player%20Character%20Object%20Reference))
  (bind _returnvalue (Transformation|GetActorLocation InteractingPlayer))
  (bind _returnvalue_2 (Transformation|GetActorTransform))
  (bind _returnvalue_3 (Math|Transform|InverseTransformLocation _returnvalue_2 _returnvalue))
  (bind _x (Math|Vector|BreakVector _returnvalue_3))
  (Utilities|IsValid InteractingPlayer
    (:Is%20Valid
      (if (> _x 1e+01)
        (return 1.0)
        (elif (< _x -1e+01)
          (return -1.0)
          (else
            (return (Variables|Default|GetOpenDirectionSign))))))
    (:Is%20Not%20Valid
      (Development|PrintString "Player Reference Missing!"))))

(fn TryOpenforEnemy
  (params (Enemy :type Actor%20Object%20Reference) (InteractingPlayer :type BP%20Player%20Character%20Object%20Reference))
  (bind _returnvalue (Transformation|GetActorLocation Enemy))
  (bind _returnvalue_2 (Transformation|GetActorTransform))
  (bind _returnvalue_3 (Math|Transform|InverseTransformLocation _returnvalue_2 _returnvalue))
  (bind _x (Math|Vector|BreakVector _returnvalue_3))
  (bind _returnvalue_4 (> _x 0.0))
  (bind _returnvalue_5 (Math|Float|SelectFloat 1.0 -1.0 _returnvalue_4))
  ;[0.15 0.15 0.15 0.5] AI may open only ordinary closed idle doors. Reuse the existing door opening, hinge animation and auto-close.
  (if (and (and (and (and (Utilities|IsValid Enemy) (Utilities|IsValid InteractingPlayer)) (Variables|Door|AI|GetAllowEnemyOpen)) (not (Variables|Default|GetIsOpen))) (not (Variables|Default|GetIsMoving)))
    (CallFunction|OnInteract InteractingPlayer)
    ;[0.15 0.15 0.15 0.5] Set the opening direction from the enemy position after reusing the standard door animation setup.
    (Variables|Default|SetOpenDirectionSign _returnvalue_5)
    (Variables|Default|SetTargetYaw (* (Variables|Door|GetOpenAngle) _returnvalue_5))
    (return true)
    (else
      (return false))))