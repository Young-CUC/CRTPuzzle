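; BP_DoorMechanism is an interactable pedestal that remotely toggles the door assigned to its TargetDoor reference.
; Its construction script keeps the parent setup and shapes ItemMesh into a scaled cube as a placeholder.
; CanInteractWith defers to the door's CanToggleFromMechanism and refuses without a valid target.
; OnInteract passes the interacting player to ToggleFromMechanism, so the door itself owns the state rules and the toggle.
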(event EventBeginPlay
  (|CallParentFunction) ; This node is disabled and will not be called.\nDrag off pins to build functionality.
)

(event Collision|EventActorBeginOverlap
  (params (OtherActor :type Actor%20Object%20Reference))
  (|CallParentFunction OtherActor) ; This node is disabled and will not be called.\nDrag off pins to build functionality.
)

(event EventTick
  (params (DeltaSeconds :type Float%20%28single-precision%29))
  (|CallParentFunction DeltaSeconds) ; This node is disabled and will not be called.\nDrag off pins to build functionality.
)

(fn ConstructionScript
  (bind _itemmesh (Variables|Default|GetItemMesh))
  ;[0.15 0.15 0.15 0.5] Keep inherited interaction range; simple pedestal placeholder for the mechanism.
  (|CallParentFunction)
  (Components|StaticMesh|SetStaticMesh _itemmesh "/Engine/BasicShapes/Cube.Cube")
  (Transformation|SetRelativeScale3D _itemmesh "(X=0.45,Y=0.45,Z=0.9)")
  (Transformation|SetRelativeLocation _itemmesh "(X=0,Y=0,Z=45)" false false))

(fn CanInteractwith
  (params (InteractingPlayer :type BP%20Player%20Character%20Object%20Reference))
  (bind _targetdoor (Variables|Mechanism|GetTargetDoor))
  ;[0.15 0.15 0.15 0.5] Only allow the mechanism when a linked door exists and is closed and stationary.
  (if (Utilities|IsValid _targetdoor)
    (return (Default|CanTogglefromMechanism _targetdoor))
    (else
      (return false))))

(fn OnInteract
  (params (InteractingPlayer :type BP%20Player%20Character%20Object%20Reference))
  (bind _targetdoor (Variables|Mechanism|GetTargetDoor))
  ;[0.15 0.15 0.15 0.5] E on the mechanism opens only its assigned TargetDoor; no per-item input handling.
  ;;[0.15 0.15 0.15 0.5] E on this mechanism toggles its linked door. Opening and closing require the mechanism.
  (if (Utilities|IsValid _targetdoor)
    (Default|TogglefromMechanism _targetdoor InteractingPlayer)))