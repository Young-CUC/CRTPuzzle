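; BP_DoubleDoor is a two-leaf door variant that extends a parent door Blueprint.
; It overrides ApplyDoorRotation to apply the supplied yaw to DoorPivot and the same rotation scaled by Opposite to DoorPivot1.
; UpdateDoorMotion only calls the parent, and the event graph holds only disabled stubs.
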(event EventBeginPlay
  (|CallParentFunction) ; This node is disabled and will not be called.\nDrag off pins to build functionality.
)

(event Collision|EventActorBeginOverlap
  (params (OtherActor :type Actor%20Object%20Reference))
  (|CallParentFunction OtherActor) ; This node is disabled and will not be called.\nDrag off pins to build functionality.
)

(event EventTick
  (params (DeltaSeconds :type Float%20%28single-precision%29))
  (|CallParentFunction DeltaSeconds) ; This node is disabled and will not be called.\nDrag off pins to build functionality.
)

(fn ConstructionScript
  (|CallParentFunction))

(fn UpdateDoorMotion
  (|CallParentFunction))

(fn ApplyDoorRotation
  (params (currentYaw :type Float%20%28double-precision%29))
  (Transformation|SetRelativeRotation (Variables|Default|GetDoorPivot) (Math|Rotator|MakeRotator 0.0 0.0 currentYaw) false false)
  (Transformation|SetRelativeRotation (Variables|Components|GetDoorPivot1) (* (Math|Rotator|MakeRotator 0.0 0.0 currentYaw) (Variables|Default|Getopposite)) false false)
  (return true))