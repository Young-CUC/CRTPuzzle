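; BP_PassWord is an interactable password lock that controls a target mechanism door.
; On interact it toggles an already open door, or creates a WBP_PasswordLock four-wheel panel with UI-only input and a visible cursor.
; A submitted code matching Code calls OpenFromMechanism and closes the panel on success; failures show feedback on the widget.
; Cancelling or success restores game-only input, and interaction is ignored while the panel is open or the door moves.
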(event Custom|InitializePasswordPanel
  (bind _passwordwidget (Variables|Default|GetPassWordWidget))
  (bind _activecontroller (Variables|Default|GetActiveController))
  ;[0.15 0.15 0.15 0.5] Open, verify, and close the four-wheel password panel
  (if (Utilities|IsValid _passwordwidget)
    (EventDispatchers|BindEventtoOnPanelCancelled _passwordwidget (delegate Custom|CustomEvent_0))
    (EventDispatchers|BindEventtoOnCodeSubmitted _passwordwidget (delegate Custom|CustomEvent))
    (UserInterface|Viewport|AddtoViewport _passwordwidget 0)
    (Input|SetInputModeUIOnly _activecontroller _passwordwidget "DoNotLock" true)
    (Variables|/Script/Engine.PlayerController|SetbShowMouseCursor _activecontroller true)
    (Variables|Default|SetisPanelOpen true)))

(event Custom|CustomEvent
  (params (EnteredCode :type String))
  (bind _passwordwidget (Variables|Default|GetPassWordWidget))
  ;[0.15 0.15 0.15 0.5] Open, verify, and close the four-wheel password panel
  (if (Utilities|Enum|Equal(Enum) EnteredCode (Variables|Default|GetCode))
    (bind _success (Default|OpenfromMechanism (Variables|Default|GetTargetDoor) (Variables|Default|GetActivePlayer)))
    (if _success
      (CallFunction|ClosePasswordPanel)
      (else
        (Default|ShowFeedback _passwordwidget "机关门不可用")))
    (else
      (Default|ShowFeedback _passwordwidget "密码错误，请重试"))))

(event Custom|CustomEvent_0
  ;[0.15 0.15 0.15 0.5] Open, verify, and close the four-wheel password panel
  (CallFunction|ClosePasswordPanel))

(event EventBeginPlay
  (|CallParentFunction) ; This node is disabled and will not be called.\nDrag off pins to build functionality.
)

(event Collision|EventActorBeginOverlap
  (params (OtherActor :type Actor%20Object%20Reference))
  (|CallParentFunction OtherActor) ; This node is disabled and will not be called.\nDrag off pins to build functionality.
)

(event EventTick
  (params (DeltaSeconds :type Float%20%28single-precision%29))
  (|CallParentFunction DeltaSeconds) ; This node is disabled and will not be called.\nDrag off pins to build functionality.
)

(fn ConstructionScript
  (|CallParentFunction))

(fn OnInteract
  (params (InteractingPlayer :type BP%20Player%20Character%20Object%20Reference))
  (Utilities|IsValid InteractingPlayer
    (:Is%20Valid
      (Utilities|IsValid (Variables|Default|GetTargetDoor)
        (:Is%20Valid
          (if (not (Variables|Default|GetisPanelOpen))
            (if (not (Variables|/Game/BluePrint/Interaction/BP_InteractableDoor.BP_InteractableDoor_C|GetIsMoving (Variables|Default|GetTargetDoor)))
              (if (Variables|/Game/BluePrint/Interaction/BP_InteractableDoor.BP_InteractableDoor_C|GetIsOpen (Variables|Default|GetTargetDoor))
                (Default|TogglefromMechanism (Variables|Default|GetTargetDoor) InteractingPlayer)
                (else
                  (bind _output_get (Variables|Default|SetActivePlayer InteractingPlayer))
                  (bind _asplayer_controller (Utilities|Casting|CastToPlayerController (Pawn|GetController _output_get)))
                  (bind _output_get_2 (Variables|Default|SetActiveController _asplayer_controller))
                  (bind _returnvalue (UserInterface|CreateWidget "/Game/BluePrint/Interaction/WBP_PasswordLock.WBP_PasswordLock_C" _output_get_2))
                  (Variables|Default|SetPassWordWidget _returnvalue)
                  (CallFunction|InitializePasswordPanel))))))))))

(fn ClosePasswordPanel
  (bind _activecontroller (Variables|Default|GetActiveController))
  (Widget|RemovefromParent (Variables|Default|GetPassWordWidget))
  (Input|SetInputModeGameOnly _activecontroller true)
  (Variables|/Script/Engine.PlayerController|SetbShowMouseCursor _activecontroller false)
  (Variables|Default|SetisPanelOpen false)
  (Variables|Default|SetPassWordWidget 0)
  (return))