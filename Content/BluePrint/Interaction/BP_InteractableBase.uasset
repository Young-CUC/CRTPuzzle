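; Base Blueprint for interactable actors that decides whether a player may interact and provides empty OnInteract behavior for children to fill in.
; TryInteract is the entry point, recording use state and time before calling OnInteract to block reentrant activation.
; CanBeInteractedWith checks enabled state, repeat policy, distance, cooldown, the overridable CanInteractWith rule and an optional visibility trace.
; The InteractionRange sphere takes its radius from InteractionDistance at construction and BeginPlay.
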(event EventBeginPlay
  (CallFunction|UpdateInteractionRange))

(event Collision|EventActorBeginOverlap
  (params (OtherActor :type Actor%20Object%20Reference)))

(event EventTick
  (params (DeltaSeconds :type Float%20%28single-precision%29)))

(fn ConstructionScript
  (CallFunction|UpdateInteractionRange))

(fn OnInteract
  (params (InteractingPlayer :type BP%20Player%20Character%20Object%20Reference)))

(fn CanInteractwith
  (params (InteractingPlayer :type BP%20Player%20Character%20Object%20Reference))
  ;[0.15 0.15 0.15 0.5] Override in children for extra requirements; base range and enabled checks remain enforced.
  (return true))

(fn CanbeInteractedwith
  (params (InteractingPlayer :type BP%20Player%20Character%20Object%20Reference))
  ;[0.15 0.15 0.15 0.5] Shared eligibility: valid player, enabled, repeat policy, exact distance, cooldown, child rule, wall occlusion.
  (if (Utilities|IsValid InteractingPlayer)
    (if (and (and (and (and (Variables|Interaction|GetCanInteract) (or (not (Variables|Default|GetHasInteracted)) (Variables|Interaction|GetCanInteractSeveral))) (<= (Transformation|GetDistanceTo InteractingPlayer) (Variables|Interaction|GetInteractionDistance))) (>= (- (Utilities|Time|GetTimeSeconds) (Variables|Default|GetLastInteractionTime)) (Math|Float|Max(Float) (Variables|Interaction|GetInteractionCooldown) 0.05))) (CallFunction|CanInteractwith InteractingPlayer))
      (if (Variables|Interaction|GetRequireLineOfSight)
        (bind _returnvalue (Collision|LineTraceByChannel (Transformation|GetActorLocation InteractingPlayer) (+ (Transformation|GetActorLocation) "0,0,50") "TraceTypeQuery1" false (Utilities|Array|MakeArray InteractingPlayer) "None"))
        (return (not _returnvalue))
        (else
          (return true)))
      (else
        _)))
  (return false))

(fn TryInteract
  (params (InteractingPlayer :type BP%20Player%20Character%20Object%20Reference))
  ;[0.15 0.15 0.15 0.5] Use this entry point. Record state BEFORE calling child OnInteract to prevent repeat/reentrant activation.
  (bind _allowed (CallFunction|CanbeInteractedwith InteractingPlayer))
  (if _allowed
    (Variables|Default|SetHasInteracted true)
    (Variables|Default|SetLastInteractionTime (Utilities|Time|GetTimeSeconds))
    (CallFunction|OnInteract InteractingPlayer)
    (return true)
    (else
      (return false))))

(fn UpdateInteractionRange
  (Components|Sphere|SetSphereRadius (Variables|Default|GetInteractionRange) (Variables|Interaction|GetInteractionDistance) true)
  (return))