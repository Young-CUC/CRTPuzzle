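; BP_ExampleSwitch is an example interactable switch, a child Blueprint that adds only custom behavior on top of inherited detection, input and validation.
; Its construction script runs the parent setup, then builds a scaled, raised cube as the item mesh.
; OnInteract increments an interaction counter, toggles IsActivated and prints the on or off state, without calling the parent implementation.
; The event graph holds only disabled default events.
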(event EventBeginPlay
  (|CallParentFunction) ; This node is disabled and will not be called.\nDrag off pins to build functionality.
)

(event Collision|EventActorBeginOverlap
  (params (OtherActor :type Actor%20Object%20Reference))
  (|CallParentFunction OtherActor) ; This node is disabled and will not be called.\nDrag off pins to build functionality.
)

(event EventTick
  (params (DeltaSeconds :type Float%20%28single-precision%29))
  (|CallParentFunction DeltaSeconds) ; This node is disabled and will not be called.\nDrag off pins to build functionality.
)

(fn ConstructionScript
  (bind _itemmesh (Variables|Default|GetItemMesh))
  ;[0.15 0.15 0.15 0.5] Inherit range setup, then build the example item mesh.
  (|CallParentFunction)
  (Components|StaticMesh|SetStaticMesh _itemmesh "/Engine/BasicShapes/Cube.Cube")
  (Transformation|SetRelativeScale3D _itemmesh "(X=0.65,Y=0.65,Z=0.8)")
  (Transformation|SetRelativeLocation _itemmesh "(X=0,Y=0,Z=40)" false false))

(fn OnInteract
  (params (InteractingPlayer :type BP%20Player%20Character%20Object%20Reference))
  ;[0.15 0.15 0.15 0.5] Example child: toggle IsActivated and increment InteractionCount; no distance or key handling here.
  ;;[0.15 0.15 0.15 0.5] Example child: only custom behavior. Detection, E input and validation are inherited/shared.
  (Variables|Default|SetInteractionCount (+ (Variables|Default|GetInteractionCount) 1))
  (Variables|Default|SetIsActivated (not (Variables|Default|GetIsActivated)))
  (Development|PrintString (Utilities|String|SelectString "Switch ON" "Switch OFF" (Variables|Default|GetIsActivated))))