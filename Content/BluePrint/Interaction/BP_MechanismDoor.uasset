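; Double-door variant that players cannot interact with directly and that only mechanisms operate remotely.
; The construction script refits the inherited frame and leaf for two 120 cm leaves.
; OpenFromMechanism only opens a closed, idle door, while ToggleFromMechanism works whenever it is not moving; both validate the player, then reuse the parent's OnInteract animation.
; Auto-close is disabled at construction, on toggle and during motion updates, which also clear its timer.
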(event EventBeginPlay
  (|CallParentFunction) ; This node is disabled and will not be called.\nDrag off pins to build functionality.
)

(event Collision|EventActorBeginOverlap
  (params (OtherActor :type Actor%20Object%20Reference))
  (|CallParentFunction OtherActor) ; This node is disabled and will not be called.\nDrag off pins to build functionality.
)

(event EventTick
  (params (DeltaSeconds :type Float%20%28single-precision%29))
  (|CallParentFunction DeltaSeconds) ; This node is disabled and will not be called.\nDrag off pins to build functionality.
)

(fn ConstructionScript
  ;[0.15 0.15 0.15 0.5] Fit frame to two 120 cm leaves: hinges -60/+180, 2 cm center gap. Inherit the double-door animation and mechanism-only access.
  (|CallParentFunction)
  (Transformation|SetRelativeLocation (Variables|Default|GetFrameRight) "(X=0,Y=189,Z=110)" false false)
  (Transformation|SetRelativeLocation (Variables|Default|GetFrameTop) "(X=0,Y=60,Z=228)" false false)
  (Transformation|SetRelativeScale3D (Variables|Default|GetFrameTop) "(X=0.22,Y=2.74,Z=0.16)")
  (Transformation|SetRelativeLocation (Variables|Default|GetDoorLeaf1) "(X=0,Y=-60,Z=110)" false false)
  (Variables|Default|SetisAutoClose false))

(fn CanInteractwith
  (params (InteractingPlayer :type BP%20Player%20Character%20Object%20Reference))
  ;[0.15 0.15 0.15 0.5] Never offer direct E interaction on this door. OpenFromMechanism is its remote entry point.
  (return false))

(fn CanOpenfromMechanism
  (return (not (or (Variables|Default|GetIsOpen) (Variables|Default|GetIsMoving)))))

(fn OpenfromMechanism
  (params (InteractingPlayer :type BP%20Player%20Character%20Object%20Reference))
  ;[0.15 0.15 0.15 0.5] Remote open only: validate player, reject open/moving doors, then reuse existing opening direction, animation and auto-close.
  (if (Utilities|IsValid InteractingPlayer)
    (if (CallFunction|CanOpenfromMechanism)
      (CallFunction|OnInteract InteractingPlayer)
      (return true)
      (else
        _)))
  (return false))

(fn CanTogglefromMechanism
  (return (not (Variables|Default|GetIsMoving))))

(fn TogglefromMechanism
  (params (InteractingPlayer :type BP%20Player%20Character%20Object%20Reference))
  ;[0.15 0.15 0.15 0.5] Mechanism-only toggle: reject invalid or busy calls, cancel old auto-close timer, disable automatic closing, then reuse the door animation.
  (if (Utilities|IsValid InteractingPlayer)
    (if (CallFunction|CanTogglefromMechanism)
      (Utilities|Time|ClearTimerbyFunctionName 0 "AutoCloseDoor")
      (Variables|Default|SetisAutoClose false)
      (CallFunction|OnInteract InteractingPlayer)
      (return true)
      (else
        _)))
  (return false))

(fn UpdateDoorMotion
  ;[0.15 0.15 0.15 0.5] Mechanism doors never schedule automatic closure. Preserve parent double-leaf motion.
  (Variables|Default|SetisAutoClose false)
  (Utilities|Time|ClearTimerbyFunctionName 0 "AutoCloseDoor")
  (|CallParentFunction))