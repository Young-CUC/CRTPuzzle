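; Camera manager actor that switches the player's view between cameras in CameraList using the 0, 1 and 2 keys.
; A key press starts a timed transition, ignored if one is running or that camera is already active.
; Tick drives ZoomY on a dynamic post-process material added to PPV, animating the view out and back in.
; At the midpoint it swaps the view target and matches control rotation to the new camera, hiding the cut.
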(event EventBeginPlay
  (Variables|Default|SetCurrentCameraID 0)
  (CallFunction|ChangeCamera)
  (Input|EnableInput (Game|GetPlayerController 0))
  (bind _returnvalue (Rendering|Material|CreateDynamicMaterialInstance (Variables|Default|Get_Material) "None" "None" :!class /Script/Engine.KismetMaterialLibrary))
  (bind _output_get (Variables|Default|SetMaterial _returnvalue))
  (Rendering|AddorUpdateBlendable (Variables|Default|GetPPV) _output_get 1.0 :!class /Script/Engine.PostProcessVolume)
  (CallFunction|Appear 1.0))

(event Collision|EventActorBeginOverlap
  (params (OtherActor :type Actor%20Object%20Reference)))

(event EventTick
  (params (DeltaSeconds :type Float%20%28single-precision%29))
  (bind _changeduration (Variables|Default|GetChangeDuration))
  (bind _returnvalue (/ _changeduration 2.0))
  (if (Variables|Default|GetIsChanging)
    (if (< (Variables|Default|Gettimer) (/ (Variables|Default|GetChangeDuration) 2.0))
      (bind _output_get (Variables|Default|Settimer (+ DeltaSeconds (Variables|Default|Gettimer))))
      (CallFunction|Appear (- 1.0 (/ _output_get (/ (Variables|Default|GetChangeDuration) 2.0))))
      (elif (< (Variables|Default|Gettimer) (Variables|Default|GetChangeDuration))
        (if (Variables|Default|GetHaveChanged)
          _
          (else
            (Variables|Default|SetHaveChanged true)
            (CallFunction|ChangeCamera)))
        (Variables|Default|Settimer (+ DeltaSeconds (Variables|Default|Gettimer)))
        (CallFunction|Appear (/ (- (Variables|Default|Gettimer) _returnvalue) _returnvalue))
        (else
          (Variables|Default|SetIsChanging false))))))

(event Input|KeyboardEvents|3
  (params (Key :type Key%20Structure)))

(event Input|KeyboardEvents|0
  (params (Key :type Key%20Structure))
  (:Pressed
    (CallFunction|KeyPressed)))

(event Input|KeyboardEvents|2
  (params (Key :type Key%20Structure))
  (:Pressed
    (CallFunction|KeyPressed 2)))

(event Input|KeyboardEvents|1
  (params (Key :type Key%20Structure))
  (:Pressed
    (CallFunction|KeyPressed 1)))

(fn ConstructionScript)

(fn KeyPressed
  (params (CameraID :type Integer))
  (if (!= CameraID (Variables|Default|GetCurrentCameraID))
    (if (not (Variables|Default|GetIsChanging))
      (Variables|Default|SetCurrentCameraID CameraID)
      (Variables|Default|SetIsChanging true)
      (Variables|Default|Settimer 0.0)
      (Variables|Default|SetHaveChanged false))))

(fn Appear
  (params (progress :type Float%20%28double-precision%29))
  (Rendering|Material|SetScalarParameterValue (Variables|Default|GetMaterial) "ZoomY" (- 1e+02 (* progress 99.0)) :!class /Script/Engine.MaterialInstanceDynamic))

(fn ChangeCamera
  (bind _cameralist (Variables|Default|GetCameraList))
  (bind _currentcameraid (Variables|Default|GetCurrentCameraID))
  (bind _output (Utilities|Array|Get(acopy) _cameralist _currentcameraid))
  (Game|Player|SetViewTargetwithBlend (Game|GetPlayerController 0) _output 0.0 "VTBlend_Linear" 0.0 false)
  (Pawn|SetControlRotation (Game|GetPlayerController 0) (Transformation|GetActorRotation _output)))