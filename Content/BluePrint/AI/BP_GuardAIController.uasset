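; Guard AI controller that runs the BB_Guard blackboard and turns perception updates into blackboard data.
; Successful hearing stimuli cache location, strength and time, then write them to the sound keys.
; Sight stimuli from the player character only set a SightCandidateVisible flag, kept in a variable and on the blackboard.
; Hearing stays separate from the player's last known position, which this controller never writes.
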(event OnTargetPerceptionUpdated(AIPerception)
  (params (Actor :type Actor%20Object%20Reference) (Stimulus :type AI%20Stimulus%20Structure))
  (bind (_age _expirationage _strength _stimuluslocation _receiverlocation _tag _bsuccessfullysensed) (Utilities|Struct|BreakAIStimulus Stimulus))
  (bind _returnvalue (Utilities|Time|GetGameTimeinSeconds))
  (bind _returnvalue_2 (Pawn|GetControlledPawn))
  (bind _returnvalue_3 (AI|GetBlackboard _returnvalue_2))
  ;[0.15 0.15 0.15 0.5] Perception callbacks cache the source stimulus location and time. Hearing never writes the reliable player LKP.
  (bind _returnvalue_4 (Class|AIPerceptionSystem|GetSenseClassforStimulus Stimulus))
  (if (== _returnvalue_4 "/Script/AIModule.AISense_Hearing")
    (if _bsuccessfullysensed
      (Variables|GuardPerception|Runtime|SetLastHeardLocation _stimuluslocation)
      (Variables|GuardPerception|Runtime|SetLastHeardStrength _strength)
      (Variables|GuardPerception|Runtime|SetLastHeardTime _returnvalue)
      (AI|Components|Blackboard|SetValueasVector _returnvalue_3 (Utilities|String|StringToName "SoundLocation") _stimuluslocation)
      (AI|Components|Blackboard|SetValueasFloat _returnvalue_3 (Utilities|String|StringToName "SoundStrength") _strength)
      (AI|Components|Blackboard|SetValueasFloat _returnvalue_3 (Utilities|String|StringToName "SoundTime") _returnvalue))
    (elif (and (== _returnvalue_4 "/Script/AIModule.AISense_Sight") (== Actor (Game|GetPlayerCharacter 0)))
      (Variables|GuardPerception|Runtime|SetSightCandidateVisible _bsuccessfullysensed)
      (AI|Components|Blackboard|SetValueasBool _returnvalue_3 (Utilities|String|StringToName "SightCandidateVisible") _bsuccessfullysensed))))

(event EventBeginPlay
  ;[0.15 0.15 0.15 0.5] Perception callbacks cache the source stimulus location and time. Hearing never writes the reliable player LKP.
  (Class|AIController|UseBlackboard "/Game/BluePrint/AI/BB_Guard.BB_Guard"))

(event EventTick
  (params (DeltaSeconds :type Float%20%28single-precision%29))
  ;[0.15 0.15 0.15 0.5] Perception callbacks cache the source stimulus location and time. Hearing never writes the reliable player LKP.
)

(fn ConstructionScript)